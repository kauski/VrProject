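; Player submarine pawn that moves, strafes, rises, sinks and yaws through custom events driven by velocity variables, with engine audio on most moves.
; Side, front and back collision overlaps disable input and play timeline-driven pushes with an alarm; top and bottom overlaps nudge it vertically.
; Separate events step down pressure and attach hull dent actors.
; A looping delay plays random spooky sounds, while Tick and timeline updates retrigger their sounds every frame.
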(event OnComponentBeginOverlap(collisionBottom)
  (params (OverlappedComponent :type Primitive%20Component%20Object%20Reference) (OtherActor :type Actor%20Object%20Reference) (OtherComp :type Primitive%20Component%20Object%20Reference) (OtherBodyIndex :type Integer) (bFromSweep :type Boolean) (SweepResult :type Hit%20Result%20Structure%20%28by%20ref%29))
  (Transformation|SetActorLocation (+ (Transformation|GetActorLocation) "0.000000,0.000000,10.000000") false false))

(event OnComponentBeginOverlap(collisionRight)
  (params (OverlappedComponent :type Primitive%20Component%20Object%20Reference) (OtherActor :type Actor%20Object%20Reference) (OtherComp :type Primitive%20Component%20Object%20Reference) (OtherBodyIndex :type Integer) (bFromSweep :type Boolean) (SweepResult :type Hit%20Result%20Structure%20%28by%20ref%29))
  (bind _returnvalue (Game|GetPlayerController 0))
  (Input|DisableInput _returnvalue)
  (bind _newtrack_0 (Timeline|Timeline_2 PlayFromStart)
    (:Update
      (Pawn|Input|AddMovementInput (Transformation|GetActorForwardVector) _newtrack_0 false)
      (Audio|PlaySound2D "/Game/Sounds/SoundEffectAlarmDamage.SoundEffectAlarmDamage" 1.0 1.0 0.0 0 0)
      (Development|PrintText (Utilities|Text|ToText(Float) _newtrack_0 "HalfToEven")))
    (:Finished
      (Input|EnableInput _returnvalue))))

(event OnComponentBeginOverlap(collisionLeft)
  (params (OverlappedComponent :type Primitive%20Component%20Object%20Reference) (OtherActor :type Actor%20Object%20Reference) (OtherComp :type Primitive%20Component%20Object%20Reference) (OtherBodyIndex :type Integer) (bFromSweep :type Boolean) (SweepResult :type Hit%20Result%20Structure%20%28by%20ref%29))
  (bind _returnvalue (Game|GetPlayerController 0))
  (Input|DisableInput _returnvalue)
  (bind _newtrack_0 (Timeline|Timeline_0 PlayFromStart)
    (:Update
      (Pawn|Input|AddMovementInput (Transformation|GetActorForwardVector) (Math|Float|Absolute(Float) _newtrack_0) false)
      (Audio|PlaySound2D "/Game/Sounds/SoundEffectAlarmDamage.SoundEffectAlarmDamage" 1.0 1.0 0.0 0 0))
    (:Finished
      (Utilities|FlowControl|Delay 0.5)
      (Input|EnableInput _returnvalue))))

(event OnComponentBeginOverlap(collisionFront)
  (params (OverlappedComponent :type Primitive%20Component%20Object%20Reference) (OtherActor :type Actor%20Object%20Reference) (OtherComp :type Primitive%20Component%20Object%20Reference) (OtherBodyIndex :type Integer) (bFromSweep :type Boolean) (SweepResult :type Hit%20Result%20Structure%20%28by%20ref%29))
  (bind _returnvalue (Game|GetPlayerController 0))
  (Input|DisableInput _returnvalue 0)
  (bind _newtrack_0 (Timeline|Timeline PlayFromStart)
    (:Update
      (Pawn|Input|AddMovementInput (Transformation|GetActorRightVector) (Math|Float|Absolute(Float) _newtrack_0) false)
      (Audio|PlaySound2D "/Game/Sounds/SoundEffectAlarmDamage.SoundEffectAlarmDamage" 1.0 1.0 0.0 0 0))
    (:Finished
      (Utilities|FlowControl|Delay 5.0)
      (Input|EnableInput _returnvalue)
      (Development|PrintText "Hello"))))

(event OnComponentBeginOverlap(collisionBack)
  (params (OverlappedComponent :type Primitive%20Component%20Object%20Reference) (OtherActor :type Actor%20Object%20Reference) (OtherComp :type Primitive%20Component%20Object%20Reference) (OtherBodyIndex :type Integer) (bFromSweep :type Boolean) (SweepResult :type Hit%20Result%20Structure%20%28by%20ref%29))
  (bind _returnvalue (Game|GetPlayerController 0))
  (Input|DisableInput _returnvalue)
  (bind _newtrack_0 (Timeline|Timeline_1 PlayFromStart)
    (:Update
      (Pawn|Input|AddMovementInput (Transformation|GetActorRightVector) _newtrack_0 false)
      (Audio|PlaySound2D "/Game/Sounds/SoundEffectAlarmDamage.SoundEffectAlarmDamage" 1.0 1.0 0.0 0 0)
      (Development|PrintText (Utilities|Text|ToText(Float) _newtrack_0 "HalfToEven")))
    (:Finished
      (Input|EnableInput _returnvalue))))

(event OnComponentBeginOverlap(collisionTop)
  (params (OverlappedComponent :type Primitive%20Component%20Object%20Reference) (OtherActor :type Actor%20Object%20Reference) (OtherComp :type Primitive%20Component%20Object%20Reference) (OtherBodyIndex :type Integer) (bFromSweep :type Boolean) (SweepResult :type Hit%20Result%20Structure%20%28by%20ref%29))
  (Transformation|SetActorLocation (+ (Transformation|GetActorLocation) "0.000000,0.000000,-10.000000") false false))

(event Custom|Forward
  (Pawn|Input|AddMovementInput (Transformation|GetActorRightVector) (Variables|Default|GetForwardBackVel) false))

(event Custom|LeftRight
  (Pawn|Input|AddMovementInput (Transformation|GetActorForwardVector) (Variables|Default|GetLeftRightVel) false)
  (Audio|PlaySound2D "/Game/Sounds/SoundEffectEngineMovement.SoundEffectEngineMovement" 1.0 1.0 0.0 0 0))

(event Custom|UpDown
  (Pawn|Input|AddMovementInput (Transformation|GetActorUpVector) (Variables|Default|GetUpDownVel) false)
  (Audio|PlaySound2D "/Game/Sounds/SoundEffectEngineMovement.SoundEffectEngineMovement" 1.0 1.0 0.0 0 0))

(event Custom|Rotate
  (Transformation|AddWorldRotation (Variables|Default|GetDefaultSceneRoot) (Math|Rotator|MakeRotator 0.0 0.0 (Variables|Default|GetRotateSpeed)) false false)
  (Audio|PlaySound2D "/Game/Sounds/SoundEffectEngineMovement.SoundEffectEngineMovement" 1.0 1.0 0.0 0 0))

(event Custom|ReleasePressure
  (if (<= (Variables|Default|GetPressure) 0.0)
    (Development|PrintString "pressure is 0")
    (else
      (bind _output_get (Variables|Default|SetPressure (- (Variables|Default|GetPressure) 25.0)))
      (Development|PrintString (Utilities|String|ToString(Float) _output_get)))))

(event Custom|HullDamage
  (params (speed :type Float%20%28double-precision%29) (Mass :type Float%20%28double-precision%29))
  (bind _returnvalue (Game|SpawnActorfromClass "/Game/Blueprints/BP_HullDent.BP_HullDent_C" (Math|Transform|MakeTransform (+ "165.340554,-0.000000,183.747863" "") "0, 0, 0" (Math|Vector|MakeVector 1.0 1.0 1.0)) "Undefined" 0 0))
  (Transformation|AttachActorToActor _returnvalue self "None" "KeepRelative" "KeepRelative" "KeepRelative" true))

(event EventBeginPlay
  (Variables|Default|SetPressure 1e+02)
  (Audio|PlaySound2D (Utilities|Select :Index (Math|Random|RandomIntegerinRange 0 5) :Option%200 "/Game/Sounds/SoundEffectSpooky1RandomIntervals.SoundEffectSpooky1RandomIntervals" :Option%201 "/Game/Sounds/SoundEffectSpooky2RandomIntervals.SoundEffectSpooky2RandomIntervals" :Option%202 "/Game/Sounds/SoundEffectSpooky3PART1RandomIntervals.SoundEffectSpooky3PART1RandomIntervals" :Option%203 "/Game/Sounds/SoundEffectSpooky3PART2RandomIntervals.SoundEffectSpooky3PART2RandomIntervals" :Option%204 "/Game/Sounds/SoundEffectSpooky4RandomIntervals.SoundEffectSpooky4RandomIntervals" :Option%205 "/Game/Sounds/SoundEffectSpooky5RandomIntervals.SoundEffectSpooky5RandomIntervals") 1e+01 1.0 0.0 0 0 :!label _label)
  (Utilities|FlowControl|Delay (Math|Conversions|ToFloat(Integer) (Math|Random|RandomIntegerinRange 45 90)))
  (goto _label))

(event EventTick
  (params (DeltaSeconds :type Float%20%28single-precision%29))
  (Audio|PlaySound2D "/Game/Sounds/Sukellussy_1.Sukellussy_1" 1.0 1.0 0.0 0 0))

(fn ConstructionScript)