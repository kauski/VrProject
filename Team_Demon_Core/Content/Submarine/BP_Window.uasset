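; Submarine window that toggles open and closed and tracks pressure exposure while open.
; WindowOpen flips the closed flag and plays or reverses a timeline that adds relative Z offsets to the cube.
; Tick uses a Delay to raise the pressure timer while open and lower it to a floor while closed.
; A cracked message prints within a threshold range; the broken check nested inside that range can never pass.
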(event Custom|WindowOpen
  (if (Variables|Default|GetWindowClosedBool)
    (Variables|Default|SetWindowClosedBool false)
    (Development|PrintText "Auki")
    (bind (_direction _open _close) (Timeline|WindowOpenTL Play)
      (:Update
        (if (Variables|Default|GetWindowClosedBool)
          (Transformation|AddRelativeLocation (Variables|Default|GetCube) (Math|Vector|MakeVector 0.0 0.0 _open) false false)
          (else
            (Transformation|AddRelativeLocation (Variables|Default|GetCube) (Math|Vector|MakeVector 0.0 0.0 _close) false false)))))
    (else
      (Variables|Default|SetWindowClosedBool true)
      (Development|PrintText "Kiinni")
      (Timeline|WindowOpenTL Reverse))))

(event EventTick
  (params (DeltaSeconds :type Float%20%28single-precision%29))
  (bind _timer (Variables|Default|GetTimer))
  (if (Variables|Default|GetWindowClosedBool)
    (Utilities|FlowControl|Delay _timer)
    (Variables|Default|SetWindowPressureTimer (- (Variables|Default|GetWindowPressureTimer) _timer))
    (if (<= (Variables|Default|GetWindowPressureTimer) 1.0)
      (bind _output_get (Variables|Default|SetWindowPressureTimer 1.0)))
    (else
      (Utilities|FlowControl|Delay _timer)
      (Variables|Default|SetWindowPressureTimer (+ (Variables|Default|GetWindowPressureTimer) _timer))
      (if (and (>= (Variables|Default|GetWindowPressureTimer) 15.0) (< (Variables|Default|GetWindowPressureTimer) 3e+01))
        (Development|PrintText "Window cracked")
        (if (>= (Variables|Default|GetWindowPressureTimer) 3e+01)
          (Development|PrintText "Window broke"))))))

(fn ConstructionScript
  (|CallParentFunction))