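; BP_SubLight is a switchable spot light that other logic can toggle through its OnOff event.
; On BeginPlay it caches the SpotLight's starting intensity as the default.
; OnOff sets the intensity to zero when the light is lit and restores the cached value otherwise, switching by intensity alone.
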(event Custom|OnOff
  (if (> (Variables|/Script/Engine.LightComponentBase|GetIntensity (Variables|Default|GetSpotLight)) 0.0)
    (Rendering|Components|Light|SetIntensity (Variables|Default|GetSpotLight) 0.0)
    (else
      (Rendering|Components|Light|SetIntensity (Variables|Default|GetSpotLight) (Variables|Default|GetdefaultIntensityVar)))))

(event EventBeginPlay
  (Variables|Default|SetdefaultIntensityVar (Variables|/Script/Engine.LightComponentBase|GetIntensity (Variables|Default|GetSpotLight))))

(fn ConstructionScript)