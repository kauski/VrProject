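; Test radar table actor that shows nearby enemies as miniature dots, positioning and attaching itself to the BP_SubPawb3 actor on BeginPlay.
; VectorTableTestScan clears old dots, then sphere-overlaps for BP_Enemy_Test pawns around the "Radari"-tagged actor.
; It converts enemy positions to table-relative vectors, flattens and scales them down, and spawns attached BP_Radar_Dot markers above the tagged actor.
; Debug spheres and prints trace the math.
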(event Custom|VectorTableTestScan
  (bind _outactors (Actor|GetAllActorswithTag "Radari"))
  (bind _outactors_2 (Actor|GetAllActorsOfClass "/Game/Blueprints/BP_Radar_Dot.BP_Radar_Dot_C"))
  (for _array_element _outactors_2
    (Actor|DestroyActor _array_element))
  (Rendering|Debug|DrawDebugSphere (Transformation|GetActorLocation (Utilities|Array|Get(acopy) _outactors)) 4e+03 24 "(R=0.034979,G=0.068063,B=0.572917,A=1.000000)" 1e+04 2.0)
  (Development|PrintString (Utilities|String|ToString(Vector) (Transformation|GetActorLocation (Utilities|Array|Get(acopy) _outactors))) true true "(R=0.000000,G=0.000000,B=0.000000,A=1.000000)")
  (Utilities|Array|Clear (Variables|Default|Getvectors))
  (bind (_outactors_3 _returnvalue) (Collision|SphereOverlapActors (Transformation|GetActorLocation (Utilities|Array|Get(acopy) _outactors)) 4e+03 (Utilities|Array|MakeArray "ObjectTypeQuery3") "/Game/Blueprints/BP_Enemy_Test.BP_Enemy_Test_C"))
  (bind _output_get (Variables|Default|SetEnemies _outactors_3))
  (if _returnvalue
    (for _array_element_2 _output_get
      (Utilities|Array|Add (Variables|Default|Getvectors) (.location (Math|Transform|MakeRelativeTransform (Transformation|GetRelativeTransform (Variables|/Script/Engine.Actor|GetRootComponent _array_element_2)) (Transformation|GetActorTransform self)))))
    (for _array_element_3 (Variables|Default|Getvectors)
      (Development|PrintString (Utilities|String|ToString(Vector) _array_element_3) true true "(R=0.463542,G=0.338397,B=0.000000,A=1.000000)")
      (bind _returnvalue_2 (Game|SpawnActorfromClass "/Game/Blueprints/BP_Radar_Dot.BP_Radar_Dot_C" (Math|Transform|MakeTransform (+ (/ (* _array_element_3 "1.000000,1.000000,0.000000") "1760.000000,1760.000000,1.000000") (Math|Vector|MakeVector (.x (Transformation|GetWorldLocation (Variables|/Script/Engine.Actor|GetRootComponent (Utilities|Array|Get(acopy) _outactors)))) (.y (Transformation|GetWorldLocation (Variables|/Script/Engine.Actor|GetRootComponent (Utilities|Array|Get(acopy) _outactors)))) (+ (.z (Transformation|GetWorldLocation (Variables|/Script/Engine.Actor|GetRootComponent (Utilities|Array|Get(acopy) _outactors)))) 4.0))) (Transformation|GetWorldRotation (Variables|Default|GetRadar_Cylinder)) "0.170000,1.000000,0.170000") "Undefined" self 0))
      (Transformation|AttachActorToActor _returnvalue_2 (Components|GetOwner (Variables|Default|GetRadar_Cylinder)) "None" "KeepWorld" "KeepWorld" "KeepWorld" false))
    (Development|PrintString "Completed" true true "(R=0.098466,G=1.000000,B=0.000000,A=1.000000)")
    (Development|PrintString (Utilities|String|ToString(Vector) (.location (Math|Transform|MakeRelativeTransform (Transformation|GetRelativeTransform (Variables|/Script/Engine.Actor|GetRootComponent _array_element_2)) (Transformation|GetActorTransform self)))) true true "(R=1.000000,G=0.784921,B=0.000000,A=1.000000)")
    (Development|PrintString (Utilities|String|ToString(Vector) (+ (/ (* _array_element_3 "1.000000,1.000000,0.000000") "1760.000000,1760.000000,1.000000") (Math|Vector|MakeVector (.x (Transformation|GetWorldLocation (Variables|/Script/Engine.Actor|GetRootComponent (Utilities|Array|Get(acopy) _outactors)))) (.y (Transformation|GetWorldLocation (Variables|/Script/Engine.Actor|GetRootComponent (Utilities|Array|Get(acopy) _outactors)))) (+ (.z (Transformation|GetWorldLocation (Variables|/Script/Engine.Actor|GetRootComponent (Utilities|Array|Get(acopy) _outactors)))) 4.0)))) true true "(R=1.000000,G=0.000000,B=0.037674,A=1.000000)")
    (Development|PrintString (Utilities|String|ToString(Vector) (Transformation|GetWorldLocation (Variables|Default|GetRadar_Cylinder))))
    (Utilities|Array|Clear (Variables|Default|Getvectors))
    (Utilities|Array|Clear (Variables|Default|GetEnemies))))

(event EventBeginPlay
  (bind _asbp_sub_pawb_3 (Utilities|Casting|CastToBP_SubPawb3Class "/Game/Submarine/BP_SubPawb3.BP_SubPawb3_C")
    (:then
      (bind _returnvalue (Actor|GetActorOfClass _asbp_sub_pawb_3))
      (Transformation|SetActorLocation (+ (Transformation|GetWorldLocation (Variables|Default|GetRadar_Cylinder)) (Math|Vector|MakeVector (+ (.x (Transformation|GetWorldLocation (Variables|/Script/Engine.Actor|GetRootComponent _returnvalue))) 3e+02) (+ (.y (Transformation|GetWorldLocation (Variables|/Script/Engine.Actor|GetRootComponent _returnvalue))) -1.8e+02) (+ (.z (Transformation|GetWorldLocation (Variables|/Script/Engine.Actor|GetRootComponent _returnvalue))) 5.7e+02))) false false)
      (Development|PrintString (Utilities|String|ToString(Vector) (+ (Transformation|GetWorldLocation (Variables|Default|GetRadar_Cylinder)) (Math|Vector|MakeVector (+ (.x (Transformation|GetWorldLocation (Variables|/Script/Engine.Actor|GetRootComponent _returnvalue))) 3e+02) (+ (.y (Transformation|GetWorldLocation (Variables|/Script/Engine.Actor|GetRootComponent _returnvalue))) -1.8e+02) (+ (.z (Transformation|GetWorldLocation (Variables|/Script/Engine.Actor|GetRootComponent _returnvalue))) 5.7e+02)))) true true "(R=0.933301,G=0.957024,B=1.000000,A=1.000000)" 1e+03)
      (Transformation|AttachActorToActor _returnvalue "None" "KeepWorld" "KeepWorld" "KeepWorld" true))
    (:CastFailed
      (Development|PrintString "Hello"))))

(event EventTick
  (params (DeltaSeconds :type Float%20%28single-precision%29)))

(fn ConstructionScript)

(fn FNAddtoRadar
  (params (Actor :type Actor%20Object%20Reference))
  (Utilities|Array|Add (Variables|Default|GetEnemies) Actor))

(fn FNRemovefromRadar
  (params (Actor :type Actor%20Object%20Reference))
  (Utilities|Array|RemoveItem (Variables|Default|GetEnemies) Actor))