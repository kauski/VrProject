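; BP_Lighting dims a directional light according to the height of the BP_SubPawb actor, apparently a submarine pawn.
; Every tick it looks up that actor and turns the light off at or below a fixed world height.
; Above that it computes intensity from the vertical gap to the light, but a second sequence step overwrites this with a constant dim value, leaving effectively a two-level switch.
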(event EventTick
  (params (DeltaSeconds :type Float%20%28single-precision%29))
  (bind _returnvalue (Actor|GetActorOfClass "/Game/Submarine/BP_SubPawb.BP_SubPawb_C"))
  (Utilities|FlowControl|Sequence
    (:then_0
      (if (<= (.z (Transformation|GetWorldLocation (Variables|/Script/Engine.Actor|GetRootComponent _returnvalue))) 2e+03)
        (Variables|Default|SetfloatVar 0.0)
        (Rendering|Components|Light|SetIntensity (Variables|Default|GetDirectionalLight) (Variables|Default|GetfloatVar))
        (else
          (Variables|Default|SetfloatVar (- 1e+01 (/ (- (.z (Transformation|GetWorldLocation (Variables|Default|GetDirectionalLight))) (.z (Transformation|GetWorldLocation (Variables|/Script/Engine.Actor|GetRootComponent _returnvalue)))) 1e+03)))
          (Rendering|Components|Light|SetIntensity (Variables|Default|GetDirectionalLight) (Variables|Default|GetfloatVar)))))
    (:then_1
      (if (>= (.z (Transformation|GetWorldLocation (Variables|/Script/Engine.Actor|GetRootComponent _returnvalue))) 2e+03)
        (Variables|Default|SetfloatVar 0.5)
        (Rendering|Components|Light|SetIntensity (Variables|Default|GetDirectionalLight) (Variables|Default|GetfloatVar))))))

(fn ConstructionScript)