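; Pressable button actor that toggles every BP_SubLight in the level through OnOff.
; It triggers from InteractwithObject or a VRPawn overlapping its Box, with IsPressed blocking re-presses.
; The press animation lowers the Cube, waits, raises it and clears the flag, using latent nodes wired inside the light loop body.
; Several disconnected debug and older toggle chains remain unused.
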(event OnComponentBeginOverlap(Box)
  (params (OverlappedComponent :type Primitive%20Component%20Object%20Reference) (OtherActor :type Actor%20Object%20Reference) (OtherComp :type Primitive%20Component%20Object%20Reference) (OtherBodyIndex :type Integer) (bFromSweep :type Boolean) (SweepResult :type Hit%20Result%20Structure%20%28by%20ref%29))
  (bind _cube (Variables|Default|GetCube))
  (bind _cube_2 (Variables|Default|GetCube))
  (bind _returnvalue (Transformation|GetRelativeTransform _cube_2))
  (bind _returnvalue_2 (Transformation|GetRelativeTransform _cube))
  (Utilities|Casting|CastToVRPawn OtherActor)
  (if (not (Variables|Default|GetisPressed))
    (Variables|Default|SetisPressed true)
    (bind _outactors (Actor|GetAllActorsOfClass "/Game/Blueprints/BP_SubLight.BP_SubLight_C"))
    (for _array_element _outactors
      (Default|OnOff _array_element)
      (Components|MoveComponentTo _cube (- (.location _returnvalue_2) "0.000000,0.000000,5.000000") (.rotation _returnvalue_2) false false 0.3 false)
      (Utilities|FlowControl|Delay 1.0)
      (Components|MoveComponentTo _cube_2 (+ (.location _returnvalue) "0.000000,0.000000,5.000000") (.rotation _returnvalue) false false 0.3 false)
      (Variables|Default|SetisPressed false))))

(event EventInteractwithObject
  (bind _cube (Variables|Default|GetCube))
  (bind _cube_2 (Variables|Default|GetCube))
  (bind _returnvalue (Transformation|GetRelativeTransform _cube_2))
  (bind _returnvalue_2 (Transformation|GetRelativeTransform _cube))
  (if (not (Variables|Default|GetisPressed))
    (Variables|Default|SetisPressed true)
    (bind _outactors (Actor|GetAllActorsOfClass "/Game/Blueprints/BP_SubLight.BP_SubLight_C"))
    (for _array_element _outactors
      (Default|OnOff _array_element)
      (Components|MoveComponentTo _cube (- (.location _returnvalue_2) "0.000000,0.000000,5.000000") (.rotation _returnvalue_2) false false 0.3 false)
      (Utilities|FlowControl|Delay 1.0)
      (Components|MoveComponentTo _cube_2 (+ (.location _returnvalue) "0.000000,0.000000,5.000000") (.rotation _returnvalue) false false 0.3 false)
      (Variables|Default|SetisPressed false))))

(fn ConstructionScript)