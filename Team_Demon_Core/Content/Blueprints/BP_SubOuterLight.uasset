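; BP_SubOuterLight is a switchable outer light fixture, built from a SpotLight and a Cylinder mesh.
; BeginPlay caches the spotlight's starting intensity as the on value.
; The OnOff event toggles by checking the current intensity, setting it to zero or back to the cached value.
; Each toggle also swaps the cylinder's material between black and emissive so the mesh matches the light state.
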(event Custom|OnOff
  (if (> (Variables|/Script/Engine.LightComponentBase|GetIntensity (Variables|Default|GetSpotLight)) 0.0)
    (Rendering|Components|Light|SetIntensity (Variables|Default|GetSpotLight) 0.0)
    (Rendering|Material|SetMaterial (Variables|Default|GetCylinder) 0 "/Game/Textures/M_Color_Black.M_Color_Black")
    (else
      (Rendering|Components|Light|SetIntensity (Variables|Default|GetSpotLight) (Variables|Default|GetdefaultIntensityVar))
      (Rendering|Material|SetMaterial (Variables|Default|GetCylinder) 0 "/Game/Textures/M_Color_EmissiveLight.M_Color_EmissiveLight"))))

(event EventBeginPlay
  (Variables|Default|SetdefaultIntensityVar (Variables|/Script/Engine.LightComponentBase|GetIntensity (Variables|Default|GetSpotLight))))

(fn ConstructionScript)