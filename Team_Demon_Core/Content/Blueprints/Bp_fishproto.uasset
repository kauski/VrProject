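; Prototype fish actor that wanders at random and homes in on the player pawn.
; On BeginPlay it glides its root over two seconds to a random offset, skewed negative on each axis, with a random rotation.
; It then checks player distance against a very large threshold: within it, it moves to the player's location and rechecks after a delay.
; Otherwise it waits and wanders again, looping through latent MoveComponentTo and Delay nodes without Tick.
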(event EventBeginPlay
  (bind _returnvalue (Transformation|GetActorLocation))
  (bind _returnvalue_2 (Math|Random|RandomFloatinRange -1e+03 1e+02))
  (bind _returnvalue_3 (Math|Random|RandomFloatinRange -1e+03 1e+02))
  (bind _returnvalue_4 (Math|Random|RandomFloatinRange -1e+03 1e+02))
  (bind _returnvalue_5 (Game|Player|GetPlayerPawn 0))
  (bind _returnvalue_6 (Transformation|GetActorLocation _returnvalue_5))
  (Components|MoveComponentTo (Variables|Default|GetDefaultSceneRoot) (Math|Vector|MakeVector (+ _returnvalue_3 (.x _returnvalue)) (+ _returnvalue_2 (.y _returnvalue)) (+ (.z _returnvalue) _returnvalue_4)) (Math|Conversions|RotationFromXVector (Math|Vector|MakeVector _returnvalue_3 _returnvalue_2 _returnvalue_4)) false false 2.0 false :!label _label)
  (if (<= (Math|Vector|Distance(Vector) (Transformation|GetActorLocation) _returnvalue_6) 1e+06) :!label _label_2
    (Components|MoveComponentTo (Variables|Default|GetDefaultSceneRoot) _returnvalue_6 "0, 0, 0" false false 2.0 false)
    (Utilities|FlowControl|Delay 3e+01)
    (goto _label_2)
    (else
      (Utilities|FlowControl|Delay 1e+01)
      (goto _label))))

(fn ConstructionScript)