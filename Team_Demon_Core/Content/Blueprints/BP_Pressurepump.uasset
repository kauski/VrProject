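; Pressure pump actor that releases pressure on the submarine pawn when its handle is pumped into a trigger.
; When Box2 is overlapped by a BP_Pumphandle, it finds BP_SubPawb by class and calls ReleasePressure, printing a debug string for other actors.
; The remaining logic is disconnected leftovers: camera-trace physics-handle grabbing and an older VRPawn-triggered press animation.
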(event OnComponentBeginOverlap(Box2)
  (params (OverlappedComponent :type Primitive%20Component%20Object%20Reference) (OtherActor :type Actor%20Object%20Reference) (OtherComp :type Primitive%20Component%20Object%20Reference) (OtherBodyIndex :type Integer) (bFromSweep :type Boolean) (SweepResult :type Hit%20Result%20Structure%20%28by%20ref%29))
  (Utilities|Casting|CastToBP_Pumphandle OtherActor
    (:then
      (bind _returnvalue (Actor|GetActorOfClass "/Game/Submarine/BP_SubPawb.BP_SubPawb_C"))
      (Default|ReleasePressure _returnvalue))
    (:CastFailed
      (Development|PrintString "huonosti men"))))

(fn ConstructionScript)