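; BP_NextLevel is a trigger box that moves the player to the Blank_Level_lightinh level.
; Any overlap creates a W_Transitions widget; if the actor is BP_FirstPersonCharacter or PB_SubPawb, both branches share one transition path.
; That path plays the fade forward, waits briefly, then opens the level.
; A reverse fade follows the open call, targeting a separate Widget reference rather than the newly created widget.
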(event OnComponentBeginOverlap(Box)
  (params (OverlappedComponent :type Primitive%20Component%20Object%20Reference) (OtherActor :type Actor%20Object%20Reference) (OtherComp :type Primitive%20Component%20Object%20Reference) (OtherBodyIndex :type Integer) (bFromSweep :type Boolean) (SweepResult :type Hit%20Result%20Structure%20%28by%20ref%29))
  (bind _returnvalue (UserInterface|CreateWidget "/Game/Blueprints/W_Transitions.W_Transitions_C" (Game|GetPlayerController 0)))
  (UserInterface|Viewport|AddtoViewport _returnvalue 0)
  (Utilities|FlowControl|Sequence
    (:then_0
      (Utilities|Casting|CastToBP_FirstPersonCharacter OtherActor))
    (:then_1
      (Utilities|Casting|CastToPB_SubPawb OtherActor)))
  (Default|TransitionFade _returnvalue "Forward" 1.0)
  (Utilities|FlowControl|Delay 3.5)
  (Development|PrintString "Meni")
  (Game|OpenLevel(byObjectReference) "/Game/Blank_Level_lightinh.Blank_Level_lightinh")
  (bind _asw_transitions (Utilities|Casting|CastToW_Transitions (Variables|Default|GetWidget)))
  (Default|TransitionFade _asw_transitions "Reverse" 1.0))

(fn ConstructionScript)