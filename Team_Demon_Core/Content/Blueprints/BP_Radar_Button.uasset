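; BP_Radar_Button is a pressable button that starts a new scan on BP_Test_VectorTable, apparently for a radar.
; InteractwithObject, guarded by IsPressed, finds the table by class and calls VectorTableTestScan.
; A VRPawn overlapping the Box also triggers the scan through the Actor reference, without checking that guard.
; Both paths share a MoveComponentTo animation that lowers and raises the button, then clears IsPressed.
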(event OnComponentBeginOverlap(Box)
  (params (OverlappedComponent :type Primitive%20Component%20Object%20Reference) (OtherActor :type Actor%20Object%20Reference) (OtherComp :type Primitive%20Component%20Object%20Reference) (OtherBodyIndex :type Integer) (bFromSweep :type Boolean) (SweepResult :type Hit%20Result%20Structure%20%28by%20ref%29))
  (bind _button (Variables|Default|GetButton))
  (bind _button_2 (Variables|Default|GetButton))
  (bind _returnvalue (Transformation|GetRelativeTransform _button))
  (bind _returnvalue_2 (Transformation|GetRelativeTransform _button_2))
  (Utilities|Casting|CastToVRPawn OtherActor)
  (bind _asbp_test_vector_table (Utilities|Casting|CastToBP_Test_VectorTable (Variables|Default|GetActor))
    (:then
      (Default|VectorTableTestScan _asbp_test_vector_table)
      (Development|PrintString "Uusi scan menee")
      (Components|MoveComponentTo _button_2 (- (.location _returnvalue_2) "0.000000,0.000000,5.000000") (.rotation _returnvalue_2) false false 0.3 false)
      (Utilities|FlowControl|Delay 1.0)
      (Components|MoveComponentTo _button (+ (.location _returnvalue) "0.000000,0.000000,5.000000") (.rotation _returnvalue) false false 1.0 false)
      (Variables|Default|SetisPressed false))
    (:CastFailed
      (Development|PrintString "ei mene"))))

(event EventInteractwithObject
  (bind _button (Variables|Default|GetButton))
  (bind _button_2 (Variables|Default|GetButton))
  (bind _returnvalue (Transformation|GetRelativeTransform _button))
  (bind _returnvalue_2 (Transformation|GetRelativeTransform _button_2))
  (if (not (Variables|Default|GetisPressed))
    (Variables|Default|SetisPressed true)
    (bind _returnvalue_3 (Actor|GetActorOfClass "/Game/Blueprints/BP_Test_VectorTable.BP_Test_VectorTable_C"))
    (Default|VectorTableTestScan _returnvalue_3)
    (Development|PrintString "Uusi scan menee")
    (Components|MoveComponentTo _button_2 (- (.location _returnvalue_2) "0.000000,0.000000,5.000000") (.rotation _returnvalue_2) false false 0.3 false)
    (Utilities|FlowControl|Delay 1.0)
    (Components|MoveComponentTo _button (+ (.location _returnvalue) "0.000000,0.000000,5.000000") (.rotation _returnvalue) false false 1.0 false)
    (Variables|Default|SetisPressed false)))

(fn ConstructionScript)