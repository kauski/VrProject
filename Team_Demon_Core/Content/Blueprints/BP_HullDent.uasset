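; BP_HullDent is an actor representing a hull dent that is removed by knocking on it three times.
; Interaction events and overlaps of Sphere1 by either the VR pawn or a BP_Hammer each increment a Knocks counter, with debug prints for each source.
; On the third knock the actor destroys itself.
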(event OnComponentBeginOverlap(Sphere1)
  (params (OverlappedComponent :type Primitive%20Component%20Object%20Reference) (OtherActor :type Actor%20Object%20Reference) (OtherComp :type Primitive%20Component%20Object%20Reference) (OtherBodyIndex :type Integer) (bFromSweep :type Boolean) (SweepResult :type Hit%20Result%20Structure%20%28by%20ref%29))
  (Utilities|FlowControl|Sequence
    (:then_0
      (Utilities|Casting|CastToVRPawn OtherActor)
      (Development|PrintString "Thru VR pawn"))
    (:then_1
      (Utilities|Casting|CastToBP_Hammer OtherActor)
      (Development|PrintString "Hammer time B)")))
  (Variables|Default|Setknocks (+ 1.0 (Variables|Default|Getknocks)))
  (if (== 3.0 (Variables|Default|Getknocks))
    (Actor|DestroyActor)
    (Variables|Default|Setknocks 0.0)))

(event EventInteractwithObject
  (Development|PrintString "kops kops")
  (Variables|Default|Setknocks (+ 1.0 (Variables|Default|Getknocks)))
  (if (== 3.0 (Variables|Default|Getknocks))
    (Actor|DestroyActor)
    (Variables|Default|Setknocks 0.0)))

(fn ConstructionScript)