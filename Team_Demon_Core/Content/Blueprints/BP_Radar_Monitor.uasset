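; BP_Radar_Monitor is a radar monitor Blueprint that takes brief scene captures of its surroundings instead of capturing continuously.
; BeginPlay enables tick on its SceneCaptureComponent2D, then disables it after a short delay, so the capture stops updating.
; The ScanSurroundings event repeats that short tick window to refresh the capture, then prints a Finnish debug message saying a button was pressed.
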(event Custom|ScanSurroundings
  (Variables|Default|SetSceneCaptureComponent2D (Variables|Default|GetSceneCaptureComponent2D))
  (Components|Tick|SetComponentTickEnabled (Variables|Default|GetSceneCaptureComponent2D) true)
  (Utilities|FlowControl|Delay 0.2)
  (Components|Tick|SetComponentTickEnabled (Variables|Default|GetSceneCaptureComponent2D) false)
  (Development|PrintString "nappulaa on painettu"))

(event EventBeginPlay
  (Components|Tick|SetComponentTickEnabled (Variables|Default|GetSceneCaptureComponent2D) true)
  (Utilities|FlowControl|Delay 0.2)
  (Components|Tick|SetComponentTickEnabled (Variables|Default|GetSceneCaptureComponent2D) false))

(fn ConstructionScript)