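; BP_Window is an interactable window that toggles open and closed on each InteractwithObject event.
; A boolean tracks the state and chooses whether to play or reverse the WindowOpenTL timeline, which drives the Cube's relative yaw.
; Each toggle also prints the new state in Finnish ("Auki" for open, "Kiinni" for closed).
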(event EventInteractwithObject
  (if (Variables|Default|GetWindowClosedBool)
    (Variables|Default|SetWindowClosedBool false)
    (Development|PrintText "Auki")
    (bind _newtrack_0 (Timeline|WindowOpenTL Play)
      (:Update
        (Transformation|SetRelativeRotation (Variables|Default|GetCube) (Math|Rotator|MakeRotator 0.0 0.0 _newtrack_0) false false)))
    (else
      (Variables|Default|SetWindowClosedBool true)
      (Development|PrintText "Kiinni")
      (Timeline|WindowOpenTL Reverse))))

(fn ConstructionScript
  (|CallParentFunction))