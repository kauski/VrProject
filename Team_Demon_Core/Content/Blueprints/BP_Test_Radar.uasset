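; Test radar actor that scans for nearby enemies and spawns dots for them on a radar cylinder.
; Key 1 or Scansurroundings runs a sphere overlap for BP_Enemy_Test pawns, with debug drawing.
; Dots use scaled-down enemy positions, centered by coordinate averages whose sums update after the loop, so lag one scan.
; Add/remove functions maintain an Enemies list the scan never reads.
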(event Custom|Scan%20surroundings
  (bind _returnvalue (Transformation|GetActorLocation))
  (bind _radar_cylinder (Variables|Default|GetRadar_Cylinder))
  (bind _returnvalue_2 (Transformation|GetWorldLocation _radar_cylinder))
  (bind (_x _y _z) (Class|KismetMathLibrary|BreakVector3f _returnvalue_2))
  (Rendering|Debug|DrawDebugSphere _returnvalue 1e+03 24 "(R=0.034979,G=0.068063,B=0.572917,A=1.000000)" 1e+04 2.0)
  (bind (_outactors _returnvalue_3) (Collision|SphereOverlapActors _returnvalue 1e+03 (Utilities|Array|MakeArray "ObjectTypeQuery3") "/Game/Blueprints/BP_Enemy_Test.BP_Enemy_Test_C"))
  (if _returnvalue_3
    (for _array_element _outactors
      (Rendering|Debug|DrawDebugBox (Transformation|GetWorldLocation (Variables|/Script/Engine.Actor|GetRootComponent _array_element)) "10.000000,10.000000,1000.000000" "(R=1.000000,G=0.736161,B=0.000000,A=1.000000)" "0, 0, 0" 1e+04 1e+01)
      (Utilities|FlowControl|Sequence
        (:then_0
          (Utilities|Array|Add (Variables|Default|GetyCoordinates) (/ (.Y (Class|KismetMathLibrary|BreakVector3f (Transformation|GetWorldLocation (Variables|/Script/Engine.Actor|GetRootComponent _array_element)))) 25.0))
          (Development|PrintString "Hello" true true "(R=0.152385,G=0.140706,B=0.473958,A=1.000000)")
          (Development|PrintString "Hello" true true "(R=0.776042,G=0.163966,B=0.738398,A=1.000000)")
          (Rendering|Debug|DrawDebugBox (+ (/ (Transformation|GetWorldLocation (Variables|/Script/Engine.Actor|GetRootComponent _array_element)) "25.000000,25.000000,1.000000") (+ (Math|Vector|MakeVector _x _y _z) (Math|Vector|MakeVector (* (/ (Variables|Default|GetsumOfX) (Utilities|Array|Length _outactors)) -1.0) (* (/ (Variables|Default|GetsumOfY) (Utilities|Array|Length _outactors)) -1.0) (* (.Z (Class|KismetMathLibrary|BreakVector3f (Transformation|GetWorldLocation (Variables|/Script/Engine.Actor|GetRootComponent _array_element)))) -1.0)))) "2.000000,2.000000,100000.000000" "(R=1.000000,G=0.000000,B=0.734682,A=1.000000)" "0, 0, 0" 1.0 2.0)
          (Game|SpawnActorfromClass "/Game/Blueprints/BP_Radar_Dot.BP_Radar_Dot_C" (Math|Transform|MakeTransform (+ (+ (/ (Transformation|GetWorldLocation (Variables|/Script/Engine.Actor|GetRootComponent _array_element)) "25.000000,25.000000,1.000000") (+ (Math|Vector|MakeVector _x _y _z) (Math|Vector|MakeVector (* (/ (Variables|Default|GetsumOfX) (Utilities|Array|Length _outactors)) -1.0) (* (/ (Variables|Default|GetsumOfY) (Utilities|Array|Length _outactors)) -1.0) (* (.Z (Class|KismetMathLibrary|BreakVector3f (Transformation|GetWorldLocation (Variables|/Script/Engine.Actor|GetRootComponent _array_element)))) -1.0)))) (Math|Vector|MakeVector 0.0 0.0 4.0)) (Transformation|GetWorldRotation (Variables|Default|GetRadar_Cylinder)) "1.000000,1.000000,1.000000") "AlwaysSpawn" 0 0))
        (:then_1
          (Utilities|Array|Add (Variables|Default|GetxCoordinates) (/ (.X (Class|KismetMathLibrary|BreakVector3f (Transformation|GetWorldLocation (Variables|/Script/Engine.Actor|GetRootComponent _array_element)))) 25.0)))))
    (Development|PrintString "completed")
    (Utilities|FlowControl|Sequence
      (:then_0
        (Utilities|AddingXvalues))
      (:then_1
        (Utilities|AddingYvalues
          (:End
            (Utilities|Array|Clear (Variables|Default|GetyCoordinates))
            (Utilities|Array|Clear (Variables|Default|GetxCoordinates))))))))

(event Input|KeyboardEvents|1
  (params (Key :type Key%20Structure :default "None"))
  (bind _returnvalue (Transformation|GetActorLocation))
  (bind _radar_cylinder (Variables|Default|GetRadar_Cylinder))
  (bind _returnvalue_2 (Transformation|GetWorldLocation _radar_cylinder))
  (bind (_x _y _z) (Class|KismetMathLibrary|BreakVector3f _returnvalue_2))
  (:Released
    (Rendering|Debug|DrawDebugSphere _returnvalue 1e+03 24 "(R=0.034979,G=0.068063,B=0.572917,A=1.000000)" 1e+04 2.0)
    (bind (_outactors _returnvalue_3) (Collision|SphereOverlapActors _returnvalue 1e+03 (Utilities|Array|MakeArray "ObjectTypeQuery3") "/Game/Blueprints/BP_Enemy_Test.BP_Enemy_Test_C"))
    (if _returnvalue_3
      (for _array_element _outactors
        (Rendering|Debug|DrawDebugBox (Transformation|GetWorldLocation (Variables|/Script/Engine.Actor|GetRootComponent _array_element)) "10.000000,10.000000,1000.000000" "(R=1.000000,G=0.736161,B=0.000000,A=1.000000)" "0, 0, 0" 1e+04 1e+01)
        (Utilities|FlowControl|Sequence
          (:then_0
            (Utilities|Array|Add (Variables|Default|GetyCoordinates) (/ (.Y (Class|KismetMathLibrary|BreakVector3f (Transformation|GetWorldLocation (Variables|/Script/Engine.Actor|GetRootComponent _array_element)))) 25.0))
            (Development|PrintString "Hello" true true "(R=0.152385,G=0.140706,B=0.473958,A=1.000000)")
            (Development|PrintString "Hello" true true "(R=0.776042,G=0.163966,B=0.738398,A=1.000000)")
            (Rendering|Debug|DrawDebugBox (+ (/ (Transformation|GetWorldLocation (Variables|/Script/Engine.Actor|GetRootComponent _array_element)) "25.000000,25.000000,1.000000") (+ (Math|Vector|MakeVector _x _y _z) (Math|Vector|MakeVector (* (/ (Variables|Default|GetsumOfX) (Utilities|Array|Length _outactors)) -1.0) (* (/ (Variables|Default|GetsumOfY) (Utilities|Array|Length _outactors)) -1.0) (* (.Z (Class|KismetMathLibrary|BreakVector3f (Transformation|GetWorldLocation (Variables|/Script/Engine.Actor|GetRootComponent _array_element)))) -1.0)))) "2.000000,2.000000,100000.000000" "(R=1.000000,G=0.000000,B=0.734682,A=1.000000)" "0, 0, 0" 1.0 2.0)
            (Game|SpawnActorfromClass "/Game/Blueprints/BP_Radar_Dot.BP_Radar_Dot_C" (Math|Transform|MakeTransform (+ (+ (/ (Transformation|GetWorldLocation (Variables|/Script/Engine.Actor|GetRootComponent _array_element)) "25.000000,25.000000,1.000000") (+ (Math|Vector|MakeVector _x _y _z) (Math|Vector|MakeVector (* (/ (Variables|Default|GetsumOfX) (Utilities|Array|Length _outactors)) -1.0) (* (/ (Variables|Default|GetsumOfY) (Utilities|Array|Length _outactors)) -1.0) (* (.Z (Class|KismetMathLibrary|BreakVector3f (Transformation|GetWorldLocation (Variables|/Script/Engine.Actor|GetRootComponent _array_element)))) -1.0)))) (Math|Vector|MakeVector 0.0 0.0 4.0)) (Transformation|GetWorldRotation (Variables|Default|GetRadar_Cylinder)) "1.000000,1.000000,1.000000") "AlwaysSpawn" 0 0))
          (:then_1
            (Utilities|Array|Add (Variables|Default|GetxCoordinates) (/ (.X (Class|KismetMathLibrary|BreakVector3f (Transformation|GetWorldLocation (Variables|/Script/Engine.Actor|GetRootComponent _array_element)))) 25.0)))))
      (Development|PrintString "completed")
      (Utilities|FlowControl|Sequence
        (:then_0
          (Utilities|AddingXvalues))
        (:then_1
          (Utilities|AddingYvalues
            (:End
              (Utilities|Array|Clear (Variables|Default|GetyCoordinates))
              (Utilities|Array|Clear (Variables|Default|GetxCoordinates)))))))))

(fn ConstructionScript)

(fn FNAddtoRadar
  (params (Actor :type Actor%20Object%20Reference))
  (Utilities|Array|Add (Variables|Default|GetEnemies) Actor))

(fn FNRemovefromRadar
  (params (Actor :type Actor%20Object%20Reference))
  (Utilities|Array|RemoveItem (Variables|Default|GetEnemies) Actor))